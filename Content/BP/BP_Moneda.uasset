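; BP_Moneda is a coin pickup that the player collects by overlapping it.
; A timeline started on BeginPlay moves the Sphere component along its relative Y axis, while Tick spins it by a fixed step each frame, independent of delta time.
; On overlap with player character 0, it calls RecolectarMonedas on BP_Gamemode, then destroys itself.
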(event EventBeginPlay
  (bind _newtrack_0 (Timeline|Timeline_0 Play)
    (:Update
      (Transformation|SetRelativeLocation (Variables|Default|GetSphere) (Math|Vector|MakeVector 0.0 _newtrack_0 0.0) false false))))

(event Collision|EventActorBeginOverlap
  (params (OtherActor :type Actor%20Object%20Reference))
  (bind _asbp_gamemode (Utilities|Casting|CastToBP_Gamemode (Game|GetGameMode)))
  (if (== OtherActor (Game|GetPlayerCharacter 0))
    (Default|RecolectarMonedas _asbp_gamemode)
    (Actor|DestroyActor)))

(event EventTick
  (params (DeltaSeconds :type Float%20%28single-precision%29))
  (Transformation|AddRelativeRotation (Variables|Default|GetSphere) "0,3.000000, 0" false false))

(fn ConstructionScript)