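; BP_GameMode is a game mode Blueprint that keeps the elapsed time and the collected coin count.
; On BeginPlay, EmpezarJuego resets Tiempo and starts a looping one-second timer by function name, which fires the Reloj event to increment Tiempo.
; RecolectarMonedas adds one to Monedas and has no caller within this Blueprint.
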(event Custom|Reloj
  (Variables|Default|SetTiempo (+ (Variables|Default|GetTiempo) 1)))

(event EventBeginPlay
  (Utilities|EmpezarJuego))

(fn ConstructionScript)

(fn RecolectarMonedas
  (Variables|Default|SetMonedas (+ (Variables|Default|GetMonedas) 1)))