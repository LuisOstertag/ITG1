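; BP_Enemigo is an enemy Actor that costs the player a life from the game mode when BP_Character overlaps it.
; A DoOnce gate, reset after a short delay, keeps one contact from removing several lives at once.
; Tick keeps calling Play on a timeline whose Movimiento track drives the Cube's relative Y location, moving the enemy sideways.
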(event EventBeginPlay)

(event Collision|EventActorBeginOverlap
  (params (OtherActor :type Actor%20Object%20Reference))
  (Utilities|Casting|CastToBP_Character OtherActor)
  (bind _asbp_gamemode (Utilities|Casting|CastToBP_Gamemode (Game|GetGameMode)))
  (Utilities|FlowControl|DoOnce false :!label _label
    (:Completed
      (Variables|/Game/BP/BP_GameMode.BP_Gamemode_C|SetVidas _asbp_gamemode (- (Variables|/Game/BP/BP_GameMode.BP_Gamemode_C|GetVidas _asbp_gamemode) 1))
      (Utilities|FlowControl|Delay 0.2)
      (goto _label Reset))))

(event EventTick
  (params (DeltaSeconds :type Float%20%28single-precision%29))
  (bind _movimiento (Timeline|Timeline_0 Play)
    (:Update
      (Transformation|SetRelativeLocation (Variables|Default|GetCube) (Math|Vector|MakeVector 0.0 _movimiento 0.0) false false))))

(fn ConstructionScript)