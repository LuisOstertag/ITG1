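; BP_Enemigo3 is a moving enemy that costs the player lives on contact.
; A Timeline started at BeginPlay offsets it from its initial location.
; When BP_Character overlaps its Box, it decrements Vidas on BP_Gamemode, using a DoOnce with delayed reset as a half-second cooldown.
; A Box hit by the character briefly activates its RadialForce component.
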(event OnComponentHit(Cube)
  (params (HitComponent :type Primitive%20Component%20Object%20Reference) (OtherActor :type Actor%20Object%20Reference) (OtherComp :type Primitive%20Component%20Object%20Reference) (NormalImpulse :type Vector :default "0, 0, 0") (Hit :type Hit%20Result%20Structure%20%28by%20ref%29)))

(event OnComponentBeginOverlap(Box)
  (params (OverlappedComponent :type Primitive%20Component%20Object%20Reference) (OtherActor :type Actor%20Object%20Reference) (OtherComp :type Primitive%20Component%20Object%20Reference) (OtherBodyIndex :type Integer) (bFromSweep :type Boolean) (SweepResult :type Hit%20Result%20Structure%20%28by%20ref%29))
  (Utilities|Casting|CastToBP_Character OtherActor)
  (bind _asbp_gamemode (Utilities|Casting|CastToBP_Gamemode (Game|GetGameMode)))
  (Utilities|FlowControl|DoOnce false :!label _label
    (:Completed
      (Variables|/Game/BP/BP_GameMode.BP_Gamemode_C|SetVidas _asbp_gamemode (- (Variables|/Game/BP/BP_GameMode.BP_Gamemode_C|GetVidas _asbp_gamemode) 1))
      (Utilities|FlowControl|Delay 0.5)
      (goto _label Reset))))

(event OnComponentHit(Box)
  (params (HitComponent :type Primitive%20Component%20Object%20Reference) (OtherActor :type Actor%20Object%20Reference) (OtherComp :type Primitive%20Component%20Object%20Reference) (NormalImpulse :type Vector :default "0, 0, 0") (Hit :type Hit%20Result%20Structure%20%28by%20ref%29))
  (Utilities|Casting|CastToBP_Character OtherActor)
  (Components|Activation|Activate (Variables|Default|GetRadialForce) false)
  (Utilities|FlowControl|Delay 0.2)
  (Components|Activation|Deactivate (Variables|Default|GetRadialForce)))

(event EventBeginPlay
  (Variables|Default|SetPosicion (Transformation|GetActorLocation))
  (bind _newtrack_0 (Timeline|Timeline_2 Play)
    (:Update
      (Transformation|SetActorLocation (+ (Variables|Default|GetPosicion) _newtrack_0) false false))))

(event Collision|EventActorBeginOverlap
  (params (OtherActor :type Actor%20Object%20Reference)))

(fn ConstructionScript)